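; Telegraphed area attack that damages overlapping actors once a countdown ends, then destroys itself.
; The construction script sizes the box and scales the decal from BoxExtent, and draws a debug box.
; BeginPlay starts the damage timer, and Tick feeds elapsed fraction into the decal material's Progress parameter.
; ClassToDamage selects the target: Dummy_Base_BP via its HealthComponent or ThirdPersonCharacter directly; other classes take no damage.
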(event `self.ReceiveBeginPlay`
  (bind _returnvalue (`DecalComponent.CreateDynamicMaterialInstance` (`self.Decal`)))
  (set `self.DynMaterialInst` _returnvalue)
  (bind _returnvalue_2 (`KismetSystemLibrary.K2_SetTimerDelegate` (delegate `DealDamageToEnemy`) (`self.TimeTillDamage`)))
  (set `self.AttackTimer` _returnvalue_2))

(event `DealDamageToEnemy`
  (bind _classtodamage (`self.ClassToDamage`))
  (bind _damagetodeal (`self.DamageToDeal`))
  (bind _overlappingactors (`PrimitiveComponent.GetOverlappingActors` (`self.Box`) _classtodamage))
  (if (== _classtodamage "/Game/ThirdPersonBP/Blueprints/Dummy_Base_BP.Dummy_Base_BP_C")
    (for _array_element _overlappingactors
      (bind _asdummy_base_bp (cast `/Game/ThirdPersonBP/Blueprints/Dummy_Base_BP` _array_element))
      (`/Game/HealthComponent.TakeDamage` (`/Game/ThirdPersonBP/Blueprints/Dummy_Base_BP.HealthComponent` _asdummy_base_bp) _damagetodeal false null))
    (`self.K2_DestroyActor`)
    (elif (== _classtodamage "/Game/ThirdPersonBP/Blueprints/ThirdPersonCharacter.ThirdPersonCharacter_C")
      (for _array_element_2 _overlappingactors
        (bind _asthird_person_character (cast `/Game/ThirdPersonBP/Blueprints/ThirdPersonCharacter` _array_element_2))
        (`/Game/ThirdPersonBP/Blueprints/ThirdPersonCharacter.TakeDamage` _asthird_person_character _damagetodeal))
      (`self.K2_DestroyActor`)
      (else
        (`self.K2_DestroyActor`)))))

(event `self.ReceiveTick`
  (params (DeltaSeconds :type "Float (single-precision)"))
  (bind _attacktimer (`self.AttackTimer`))
  (if (`KismetSystemLibrary.K2_IsValidTimerHandle` _attacktimer)
    (`MaterialInstanceDynamic.SetScalarParameterValue` (`self.DynMaterialInst`) "Progress" (- 1.0 (/ (`KismetSystemLibrary.K2_GetTimerRemainingTimeHandle` _attacktimer) (`self.TimeTillDamage`))))))

(fn `UserConstructionScript`
  (bind _box (`self.Box`))
  (bind _boxextent (`self.BoxExtent`))
  (bind (_returnvalue_x _returnvalue_y _returnvalue_z) (`KismetMathLibrary.BreakVector` (/ _boxextent (50.0 50.0 50.0))))
  (`BoxComponent.SetBoxExtent` _box _boxextent true)
  (`SceneComponent.SetWorldScale3D` (`self.Decal`) (`KismetMathLibrary.MakeVector` (/ _returnvalue_z 2.0) _returnvalue_y _returnvalue_x))
  (`KismetSystemLibrary.DrawDebugBox` (`SceneComponent.K2_GetComponentLocation` _box) _boxextent (struct :`R` 1.0 :`A` 1.0) (`self.K2_GetActorRotation`) 5.0 5.0))