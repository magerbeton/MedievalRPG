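; Spawn platform actor that destroys itself shortly after the TPC actor moves away from where it started.
; BeginPlay caches TPC's location, and Tick compares the current location against it using a distance threshold.
; Once past the threshold, a Gate leads to a short Delay and DestroyActor.
; The Gate closes on exit but reopens in the same tick, so the latent Delay absorbs repeated triggers.
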(event `self.ReceiveBeginPlay`
  (set `self.InitialLocation` (`self.K2_GetActorLocation` (`self.TPC`))))

(event `self.ReceiveTick`
  (params (DeltaSeconds :type "Float (single-precision)"))
  (if (> (`KismetMathLibrary.Vector_Distance` (`self.K2_GetActorLocation` (`self.TPC`)) (`self.InitialLocation`)) 500.0)
    (`|ExecutionSequence`
      (:`then_0`
        (`/Engine/EditorBlueprintResources/StandardMacros.Gate` true :!label _label
          (:`Exit`
            (`|ExecutionSequence`
              (:`then_0`
                (`KismetSystemLibrary.Delay` 2.0)
                (`self.K2_DestroyActor`))
              (:`then_1`
                (goto _label :!via `Close`))))))
      (:`then_1`
        (goto _label :!via `Open`)))))

(fn `UserConstructionScript`)