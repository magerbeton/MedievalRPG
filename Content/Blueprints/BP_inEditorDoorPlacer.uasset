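; BP_inEditorDoorPlacer is a helper actor, named for in-editor use, that populates houses with door meshes.
; Its PopulateDoors event scans every StaticMeshActor whose first tag is "HouseWithDoor" for mesh sockets with "Door" in their names.
; At each matching socket's location and rotation, it spawns a unit-scale StaticMeshActor and assigns it the MBS_City_Door mesh.
; It does not check for or remove existing doors.
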(event `PopulateDoors`
  (bind _outactors (`GameplayStatics.GetAllActorsOfClass` "/Script/Engine.StaticMeshActor"))
  (for _array_element _outactors
    (if (== (`|GetArrayItem` (`Actor.Tags` _array_element)) "HouseWithDoor")
      (bind _staticmeshcomponent (`StaticMeshActor.StaticMeshComponent` _array_element))
      (for _array_element_2 (`SceneComponent.GetAllSocketNames` _staticmeshcomponent)
        (if (!= (`KismetStringLibrary.FindSubstring` (`KismetStringLibrary.Conv_NameToString` _array_element_2) "Door") -1)
          (bind _returnvalue (`|SpawnActorFromClass` "/Script/Engine.StaticMeshActor" (`KismetMathLibrary.MakeTransform` (`SceneComponent.GetSocketLocation` _staticmeshcomponent _array_element_2) (`SceneComponent.GetSocketRotation` _staticmeshcomponent _array_element_2) (1.0 1.0 1.0)) "Undefined" "OverrideRootScale" null null))
          (`StaticMeshComponent.SetStaticMesh` (`StaticMeshActor.StaticMeshComponent` _returnvalue) "/Game/Geometry/Meshes/MBS_CityHouses/StaticMeshes/MBS_City_Door.MBS_City_Door"))))))

(fn `UserConstructionScript`)