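; BP_QuestUpdater_Location is a placeable actor that attempts a quest update when the player character reaches its location.
; On actor overlap it casts the other actor to ThirdPersonCharacter and passes it to TryUpdateQuest, ignoring anything else.
; The construction script runs the parent's, then applies a configurable static mesh and sets its world rotation to a yaw-only value.
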(event `self.ReceiveActorBeginOverlap`
  (params (OtherActor :type "Actor Object Reference"))
  (bind _asthird_person_character (cast `/Game/ThirdPersonBP/Blueprints/ThirdPersonCharacter` OtherActor))
  (`self.TryUpdateQuest` _asthird_person_character))

(fn `UserConstructionScript`
  (bind _staticmesh (`self.StaticMesh`))
  (`parent.UserConstructionScript`)
  (`StaticMeshComponent.SetStaticMesh` _staticmesh (`self.StaticMesh_ref`))
  (`SceneComponent.K2_SetWorldRotation` _staticmesh (`KismetMathLibrary.MakeRotator` 0.0 0.0 (`self.RotationOfMesh`)) false false))