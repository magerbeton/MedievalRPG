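; BP_QuestUpdater advances a player's active quest by one step when that quest is at the stage this updater represents.
; TryUpdateQuest takes a player controller reference and casts its PlayerState to ThirdPersonPlayerState.
; If the active quest's data table and progress match QuestDataTable and QuestID, it increments progress and calls the player state's update and progress quest functions.
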(event `TryUpdateQuest`
  (params (TPC_ref :type "/Game/ThirdPersonBP/Blueprints/ThirdPersonCharacter Object Reference"))
  ;[1 1 1] Trys to update the quest when its in the slot of active quests
  (bind _asthird_person_player_state (cast `/Game/ThirdPersonBP/Blueprints/ThirdPersonPlayerState` (`Pawn.PlayerState` TPC_ref)))
  (bind (_datatable _progress) (break `/Game/QuestSystem/ActiveQuests_struct` (`/Game/ThirdPersonBP/Blueprints/ThirdPersonPlayerState.ActiveQuest` _asthird_person_player_state)))
  (if (and (== _datatable (`self.QuestDataTable`)) (== _progress (`self.QuestID`)))
    (bind _output_get (set `/Game/ThirdPersonBP/Blueprints/ThirdPersonPlayerState.ActiveQuest` (make `/Game/QuestSystem/ActiveQuests_struct` _datatable (+ _progress 1)) _asthird_person_player_state))
    (`/Game/ThirdPersonBP/Blueprints/ThirdPersonPlayerState.UpdateQuest` _asthird_person_player_state _output_get)
    (`/Game/ThirdPersonBP/Blueprints/ThirdPersonPlayerState.ProgressQuest` _asthird_person_player_state 0.0)))

(fn `UserConstructionScript`)