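; Quest reward actor that grants items to a player when their character overlaps it and the player state reports no active quest.
; It reads the last row of the ActiveQuest data table from ThirdPersonPlayerState and loops over that row's item entries.
; Each entry is created and picked up through player state functions, and the pickup result is printed.
; Nothing here destroys the actor or records that the reward was claimed.
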(event `self.ReceiveActorBeginOverlap`
  (params (OtherActor :type "Actor Object Reference"))
  (bind _asthird_person_character (cast `/Game/ThirdPersonBP/Blueprints/ThirdPersonCharacter` OtherActor))
  (bind _asthird_person_player_state (cast `/Game/ThirdPersonBP/Blueprints/ThirdPersonPlayerState` (`Pawn.PlayerState` _asthird_person_character)))
  (bind _returnvalue (`/Game/ThirdPersonBP/Blueprints/ThirdPersonPlayerState.f_IsAnyQuestActive` _asthird_person_player_state))
  (if (not _returnvalue)
    (bind _datatable (break `/Game/QuestSystem/ActiveQuests_struct` (`/Game/ThirdPersonBP/Blueprints/ThirdPersonPlayerState.ActiveQuest` _asthird_person_player_state)))
    (bind _outrownames (`DataTableFunctionLibrary.GetDataTableRowNames` _datatable))
    (bind _returnvalue_2 (`|GetDataTableRow` _datatable (`|GetArrayItem` _outrownames (- (`KismetArrayLibrary.Array_Length` _outrownames) 1)))
      (:`then`
        (for _array_element (`.ItemStruct_26_88703869444CE24679A8469B7C8DF52F` (break `/Game/QuestSystem/Quest_Struct` _returnvalue_2))
          (bind _iteminventory_struct (`/Game/ThirdPersonBP/Blueprints/ThirdPersonPlayerState.f_CreateItem` _asthird_person_player_state (break `/Game/Inventory/ItemInventory_struct` _array_element) (`.Amount_8_9696621F43A053C92E9A1689D5E34214` (break `/Game/Inventory/ItemInventory_struct` _array_element)) (`.Quality_12_07DAD0F745F28520FBA068B3443702D3` (break `/Game/Inventory/ItemInventory_struct` _array_element))))
          (bind _info (`/Game/ThirdPersonBP/Blueprints/ThirdPersonPlayerState.f_Pickup` _asthird_person_player_state _iteminventory_struct))
          (`KismetSystemLibrary.PrintText` _info))))))

(fn `UserConstructionScript`)