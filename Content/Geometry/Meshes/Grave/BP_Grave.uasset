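; BP_Grave is a gravestone Blueprint that varies its look in the Construction Script.
; It creates a dynamic material instance of the rock front panel material on Grave01's second material slot.
; The panel's Texture parameter takes SpecialTexture when set, otherwise a random pick from AllGraveTextures.
; It then assigns Grave01 a random static mesh from AllStaticMeshes.
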(fn `UserConstructionScript`
  (bind _grave01 (`self.Grave01`))
  (bind _specialtexture (`self.SpecialTexture`))
  (bind _returnvalue (`PrimitiveComponent.CreateDynamicMaterialInstance` _grave01 1 "/Game/Geometry/Meshes/Grave/Grave_RockFrontpannel.Grave_RockFrontpannel" "None"))
  (`MaterialInstanceDynamic.SetTextureParameterValue` _returnvalue "Texture" (select `bool` (`KismetSystemLibrary.IsValid` _specialtexture) :`false` (`/Engine/EditorBlueprintResources/StandardMacros.RandomElementFromArrayWithIndex` (`self.AllGraveTextures`)) :`true` _specialtexture))
  (`StaticMeshComponent.SetStaticMesh` _grave01 (`/Engine/EditorBlueprintResources/StandardMacros.RandomElementFromArrayWithIndex` (`self.AllStaticMeshes`))))