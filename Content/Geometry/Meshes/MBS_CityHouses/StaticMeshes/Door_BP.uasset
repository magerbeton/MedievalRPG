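; Door Blueprint that swings its static mesh between a closed rotation and one yawed -90 degrees from it.
; BeginPlay stores the starting world rotation as closed; OpenDoor sets the target state, and ChangeDoorstate toggles it.
; OpenDoor opens a Gate that lets Tick ease the mesh toward the target with RInterpTo.
; The Gate closes once the rotation is within tolerance, ending the movement.
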(event `ChangeDoorstate`
  (`self.OpenDoor` (not (`self.DoorOpen`))))

(event `self.ReceiveBeginPlay`
  (set `self.DoorRotation_Base` (`SceneComponent.K2_GetComponentRotation` (`self.StaticMesh`))))

(event `OpenDoor`
  (params (bPickA :type Boolean))
  (bind _doorrotation_base (`self.DoorRotation_Base`))
  (bind _returnvalue (`SceneComponent.K2_GetComponentRotation` (`self.StaticMesh`)))
  (bind _returnvalue_2 (`KismetMathLibrary.SelectRotator` (`KismetMathLibrary.MakeRotator` (.roll _doorrotation_base) (.pitch _doorrotation_base) (- (.yaw _doorrotation_base) 90.0)) _doorrotation_base (`self.DoorOpen`)))
  (set `self.DoorOpen` bPickA)
  (set `self.DoorRotation` (struct))
  (goto _label :!via `Open`))

(event `self.ReceiveTick`
  (params (DeltaSeconds :type "Float (single-precision)"))
  (bind _doorrotation_base (`self.DoorRotation_Base`))
  (bind _returnvalue (`SceneComponent.K2_GetComponentRotation` (`self.StaticMesh`)))
  (bind _returnvalue_2 (`KismetMathLibrary.SelectRotator` (`KismetMathLibrary.MakeRotator` (.roll _doorrotation_base) (.pitch _doorrotation_base) (- (.yaw _doorrotation_base) 90.0)) _doorrotation_base (`self.DoorOpen`)))
  (`/Engine/EditorBlueprintResources/StandardMacros.Gate` false :!label _label
    (:`Exit`
      (if (!= _returnvalue _returnvalue_2 :`ErrorTolerance` 0.5)
        (`SceneComponent.K2_SetWorldRotation` (`self.StaticMesh`) (`KismetMathLibrary.RInterpTo` _returnvalue _returnvalue_2 DeltaSeconds 3.0) false false)
        (else
          (`self.StopDoorMovement`))))))

(event `StopDoorMovement`
  (goto _label :!via `Close`))

(fn `UserConstructionScript`)