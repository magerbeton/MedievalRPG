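; A quest-relevant city wall gate that opens when a player with the matching active quest step reaches its trigger.
; Overlapping the Box reads the character's ThirdPersonPlayerState and compares the active quest's datatable and progress against the gate's QuestStruct and Index.
; A match sets GateOpen and calls FCompletedQuest, while a mismatch closes the gate; both then call UpdateGateVis.
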(event `self.Box.OnComponentBeginOverlap`
  (params (OverlappedComponent :type "PrimitiveComponent Object Reference") (OtherActor :type "Actor Object Reference") (OtherComp :type "PrimitiveComponent Object Reference") (OtherBodyIndex :type Integer) (bFromSweep :type Boolean) (SweepResult :type "HitResult Structure (by ref)"))
  (bind _asthird_person_character (cast `/Game/ThirdPersonBP/Blueprints/ThirdPersonCharacter` OtherActor))
  (bind _asthird_person_player_state (cast `/Game/ThirdPersonBP/Blueprints/ThirdPersonPlayerState` (`Pawn.PlayerState` _asthird_person_character)))
  (bind (_activequest_datatable _activequest_progress) (break `/Game/QuestSystem/ActiveQuests_struct` (`/Game/ThirdPersonBP/Blueprints/ThirdPersonPlayerState.ActiveQuest` _asthird_person_player_state)))
  (if (and (== _activequest_datatable (`self.QuestStruct`)) (== _activequest_progress (`self.Index`)))
    (set `self.GateOpen?` true)
    (`/Game/ThirdPersonBP/Blueprints/ThirdPersonPlayerState.f_CompletedQuest` _asthird_person_player_state)
    (else
      (set `self.GateOpen?` false)))
  (`self.UpdateGateVis`))

(fn `UserConstructionScript`
  (`parent.UserConstructionScript`))