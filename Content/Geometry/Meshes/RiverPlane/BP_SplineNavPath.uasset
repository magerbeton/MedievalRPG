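; BP_SplineNavPath is a spline path actor with a utility event, AllignToFloor, that snaps its points onto the landscape.
; The event runs a long vertical Visibility trace through each point, drawing debug lines and printing the hit actor's class.
; Points move to the impact only when the first hit is a Landscape or LandscapeStreamingProxy, then the spline updates.
; Nothing else in the graphs has logic.
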(event `AllignToFloor`
  (bind _spline (`self.Spline`))
  (for _index (range (`SplineComponent.GetNumberOfSplinePoints` _spline))
    (bind _returnvalue (`SplineComponent.GetLocationAtSplinePoint` _spline _index "World"))
    (bind (_outhit _returnvalue_2) (`KismetSystemLibrary.LineTraceSingle` :`Start` (+ _returnvalue (0.0 0.0 100000.0)) :`End` (- _returnvalue (0.0 0.0 1000000.0)) :`TraceChannel` "TraceTypeQuery1" :`DrawDebugType` "ForDuration"))
    (if _returnvalue_2
      (bind (_bblockinghit _binitialoverlap _time _distance _location _impactpoint _normal _impactnormal _physmat _hitactor) (`GameplayStatics.BreakHitResult` _outhit))
      (bind _returnvalue_3 (`GameplayStatics.GetObjectClass` _hitactor))
      (`KismetSystemLibrary.PrintString` (`KismetSystemLibrary.GetClassDisplayName` _returnvalue_3))
      (if (or (== _returnvalue_3 "/Script/Landscape.LandscapeStreamingProxy") (== _returnvalue_3 "/Script/Landscape.Landscape"))
        (`SplineComponent.SetLocationAtSplinePoint` _spline _index _impactpoint "World" true))))
  (`SplineComponent.UpdateSpline` _spline))

(fn `UserConstructionScript`)