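; BP_WeaponRack is a weapon rack actor that randomizes the parts of its displayed weapons, with all logic in the Construction Script.
; It loops over eight static mesh components and reads each one's first component tag: Klinge (blade), Parierstange (crossguard), Griff (grip) or Knauf (pommel).
; Each component gets a random mesh from the matching part array, re-rolled whenever construction reruns.
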(fn `UserConstructionScript`
  (for _array_element (`|MakeArray` (`self.StaticMesh2`) (`self.StaticMesh3`) (`self.StaticMesh4`) (`self.StaticMesh5`) (`self.StaticMesh6`) (`self.StaticMesh7`) (`self.StaticMesh8`) (`self.StaticMesh1`))
    (switch `name` (`|GetArrayItem` (`ActorComponent.ComponentTags` _array_element))
      (:`klinge`
        (`StaticMeshComponent.SetStaticMesh` _array_element (`/Engine/EditorBlueprintResources/StandardMacros.RandomElementFromArrayWithIndex` (`self.Klingen`))))
      (:`parierstange`
        (`StaticMeshComponent.SetStaticMesh` _array_element (`/Engine/EditorBlueprintResources/StandardMacros.RandomElementFromArrayWithIndex` (`self.parierstangen`))))
      (:`griff`
        (`StaticMeshComponent.SetStaticMesh` _array_element (`/Engine/EditorBlueprintResources/StandardMacros.RandomElementFromArrayWithIndex` (`self.Griffe`))))
      (:`knauf`
        (`StaticMeshComponent.SetStaticMesh` _array_element (`/Engine/EditorBlueprintResources/StandardMacros.RandomElementFromArrayWithIndex` (`self.Knäufe`)))))))