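; BP_DialogActor is an NPC actor for the dialog system, with an optional skeletal mesh override applied in the construction script.
; On BeginPlay it generates a name: if the last Dialogue row reads "RNDM", it picks a Babynames entry using its truncated location coordinates, giving a repeatable pseudo-random result.
; Timer-driven distance culling against the GameInstance's player location is present but disconnected, and FGiveRandomName is an empty stub.
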(event `self.ReceiveBeginPlay`
  (`self.f_CheckForVisibilityDistance`)
  (`self.f_GenerateName`))

(fn `f_CheckForVisibilityDistance`)

(fn `f_GenerateName`
  (returns (name :type Text))
  (bind _dialogue (`self.Dialogue`))
  (bind _outrownames (`DataTableFunctionLibrary.GetDataTableRowNames` _dialogue))
  (bind _returnvalue (- (`KismetArrayLibrary.Array_Length` _outrownames) 1))
  (if (not (< _returnvalue 0))
    (bind _returnvalue_2 (`|GetDataTableRow` _dialogue (`|GetArrayItem` _outrownames _returnvalue))
      (:`then`
        (if (`KismetTextLibrary.EqualEqual_TextText` (`.Inhalt_31_F782D0A74D11B36FB641AB8894A5A1D1` (break `/Game/DialogSystem/Dialog_struct` _returnvalue_2)) "RNDM")
          (bind _outrownames_2 (`DataTableFunctionLibrary.GetDataTableRowNames` "/Game/DialogSystem/baby-names.baby-names"))
          (bind _returnvalue_3 (mod (+ (`KismetMathLibrary.FTrunc` (.x (`self.K2_GetActorLocation`))) (`KismetMathLibrary.FTrunc` (.y (`self.K2_GetActorLocation`))) (`KismetMathLibrary.FTrunc` (.z (`self.K2_GetActorLocation`)))) (- (`KismetArrayLibrary.Array_Length` _outrownames_2) 1)))
          (`KismetSystemLibrary.PrintString` (`KismetStringLibrary.Conv_IntToString` _returnvalue_3))
          (bind _returnvalue_4 (`|GetDataTableRow` "/Game/DialogSystem/baby-names.baby-names" (`|GetArrayItem` _outrownames_2 _returnvalue_3))
            (:`then`
              (bind (_year _name) (break `/Game/DialogSystem/RandomNameList_Struct` _returnvalue_4))
              (bind _output_get (set `self.NPC_Name` _name))
              (`KismetSystemLibrary.PrintString` (`KismetTextLibrary.Conv_TextToString` _output_get))
              (return _name))))))))

(fn `f_GiveRandomName`)

(fn `UserConstructionScript`
  (bind _newskeletalmesh (`self.NewSkeletalMesh`))
  (`/Engine/EditorBlueprintResources/StandardMacros.IsValid` _newskeletalmesh
    (:`Is Valid`
      (`SkinnedMeshComponent.SetSkinnedAssetAndUpdate` (`self.SkeletalMesh`) _newskeletalmesh true))))