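; Lootable actor that holds randomly generated item loot and destroys itself on a decay timer started at BeginPlay.
; GenerateLoot fills the inventory from a data table, rolling each row's drop chance and amount, with quality shaped by a curve across the row's range.
; An empty result rerolls recursively up to a counter cap when loot is forced, and otherwise destroys the actor.
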(event `self.ReceiveBeginPlay`
  (`KismetSystemLibrary.K2_SetTimerDelegate` (delegate `Decayed`) 120.0))

(event `GenerateLoot`
  (set `self.Counter` 0)
  (`self.f_FillInventory` true))

(event `Decayed`
  (`self.K2_DestroyActor`))

(fn `f_FillInventory`
  (params (`Force to have loot` :type Boolean))
  (bind _loottable (`self.Loottable`))
  (`KismetArrayLibrary.Array_Clear` (`self.Inventory`))
  (bind _outrownames (`DataTableFunctionLibrary.GetDataTableRowNames` _loottable))
  (for _array_element _outrownames
    (bind _returnvalue (`|GetDataTableRow` _loottable _array_element)
      (:`then`
        (bind (_id _droppercentage _rangeofquality _rangeofamount) (break `/Game/Inventory/Lootable/Loottables/Lootable_Struct` _returnvalue))
        (if (<= (`KismetMathLibrary.RandomFloat`) _droppercentage)
          (bind _output (`|GetArrayItem` _rangeofquality))
          (bind _iteminventory_struct (`/Game/ThirdPersonBP/Blueprints/InventoryFunctionLib.Create Item` _id (`KismetMathLibrary.RandomIntegerInRange` (`|GetArrayItem` _rangeofamount) (`|GetArrayItem` _rangeofamount 1)) (`KismetMathLibrary.Round` (+ (* (`KismetMathLibrary.Abs_Int` (- _output (`|GetArrayItem` _rangeofquality 1))) (`CurveFloat.GetFloatValue` (`self.QualityCurve`) (`KismetMathLibrary.RandomFloat`))) (`KismetMathLibrary.Conv_IntToDouble` _output))) (`/Engine/EditorBlueprintResources/StandardMacros.makeEmptyArray`)))
          (`KismetArrayLibrary.Array_Add` (`self.Inventory`) _iteminventory_struct)))))
  (if (> (`self.Counter`) 25)
    (return)
    (elif (== (`KismetArrayLibrary.Array_Length` (`self.Inventory`)) 0)
      (if `Force to have loot`
        (`/Engine/EditorBlueprintResources/StandardMacros.IncrementInt` (`self.Counter`)
          (:`  `
            (`self.f_FillInventory` `Force to have loot`)))
        (else
          (`self.K2_DestroyActor`)))
      (else
        (return)))))

(fn `UserConstructionScript`)